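; Purchasable door Blueprint that the player unlocks by spending points with the F key.
; Overlap events track the RU74 player character and toggle its Interaction flag, though end overlap re-evaluates the same comparison, so Overlap stays true after leaving.
; With Overlap set and enough points, F calls OpenDoor, hides the door, disables its collision and deducts RequiredPoints.
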(event EventBeginPlay
  ;[1 1 1] Allowing Door blueprint to trigger off keyboard press
  (Input|EnableInput (Game|GetPlayerController 0)))

(event EventTick
  (params (DeltaSeconds :type Float%20%28single-precision%29)))

(event Collision|EventActorBeginOverlap
  (params (OtherActor :type Actor%20Object%20Reference))
  (bind _returnvalue (Game|GetPlayerCharacter 0))
  (bind _asbp_ru74_character (Utilities|Casting|CastToBP_RU74_Character _returnvalue))
  (bind _returnvalue_2 (== OtherActor _asbp_ru74_character))
  ;[1 1 1] Checking if overlap
  (if _returnvalue_2
    (Variables|Default|SetOverlapPlayer OtherActor)
    (Variables|Default|SetOverlap _returnvalue_2)
    (Variables|/Game/FPS_Assault_Pack/Blueprints/RU74/BP_RU74_Character.BP_RU74_Character_C|SetInteraction _asbp_ru74_character true)))

(event Collision|EventActorEndOverlap
  (params (OtherActor :type Actor%20Object%20Reference))
  (bind _returnvalue (Game|GetPlayerCharacter 0))
  (bind _asbp_ru74_character (Utilities|Casting|CastToBP_RU74_Character _returnvalue))
  (bind _returnvalue_2 (== OtherActor _asbp_ru74_character))
  ;[1 1 1] Checking if overlap
  (if _returnvalue_2
    (Variables|Default|SetOverlapPlayer 0)
    (Variables|Default|SetOverlap _returnvalue_2)
    (Variables|/Game/FPS_Assault_Pack/Blueprints/RU74/BP_RU74_Character.BP_RU74_Character_C|SetInteraction _asbp_ru74_character false)))

(event Input|KeyboardEvents|F
  (params (Key :type Key%20Structure :default "None"))
  (:Pressed
    (bind _asbp_ru74_character (Utilities|Casting|CastToBP_RU74_Character (Game|GetPlayerCharacter 0)))
    (if (Variables|Default|GetOverlap)
      ;[1 1 1] This is what will check for points
      (if (>= (Variables|/Game/FPS_Assault_Pack/Blueprints/RU74/BP_RU74_Character.BP_RU74_Character_C|GetPoints _asbp_ru74_character) (Variables|Default|GetRequiredPoints))
        (Default|CallOpenDoor)
        ;[1 1 1] Get rid of door
        (Rendering|SetActorHiddenInGame true)
        (Collision|SetActorEnableCollision false)
        ;[1 1 1] Remove points
        (Variables|/Game/FPS_Assault_Pack/Blueprints/RU74/BP_RU74_Character.BP_RU74_Character_C|SetPoints _asbp_ru74_character (- (Variables|/Game/FPS_Assault_Pack/Blueprints/RU74/BP_RU74_Character.BP_RU74_Character_C|GetPoints _asbp_ru74_character) (Variables|Default|GetRequiredPoints)))))))

(fn ConstructionScript)