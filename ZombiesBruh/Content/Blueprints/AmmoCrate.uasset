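; AmmoCrate is a purchasable ammo pickup that sells spare ammo for player points.
; Begin and end overlap toggle an Overlap flag and the character's Interaction flag, comparing against a BP_RU74_Character reference that is fetched only when F is pressed.
; With input enabled on BeginPlay, F adds ammo to the current WeaponInv entry and deducts points if overlapping, below max reserve and affordable.
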(event EventBeginPlay
  ;[1 1 1] Enable input
  (Input|EnableInput (Game|GetPlayerController 0)))

(event Collision|EventActorBeginOverlap
  (params (OtherActor :type Actor%20Object%20Reference))
  ;[1 1 1] Checking if overlap
  (if (== OtherActor (stale Input|KeyboardEvents|F _returnvalue))
    (Variables|Default|SetOverlap true)
    (Variables|/Game/FPS_Assault_Pack/Blueprints/RU74/BP_RU74_Character.BP_RU74_Character_C|SetInteraction (stale Input|KeyboardEvents|F _returnvalue) true)))

(event Collision|EventActorEndOverlap
  (params (OtherActor :type Actor%20Object%20Reference))
  ;[1 1 1] Checking if overlap
  (if (== OtherActor (stale Input|KeyboardEvents|F _returnvalue))
    (Variables|Default|SetOverlap false)
    (Variables|/Game/FPS_Assault_Pack/Blueprints/RU74/BP_RU74_Character.BP_RU74_Character_C|SetInteraction (stale Input|KeyboardEvents|F _returnvalue) false)))

(event Input|KeyboardEvents|F
  (params (Key :type Key%20Structure :default "None"))
  (bind _requiredpoints (Variables|Default|GetRequiredPoints))
  ;[1 1 1] Reference player on F
  (:Pressed
    (bind _returnvalue (Actor|GetActorOfClass "/Game/FPS_Assault_Pack/Blueprints/RU74/BP_RU74_Character.BP_RU74_Character_C"))
    (if (not (>= (Utilities|Struct|BreakWeaponsInfo (Utilities|Array|Get(acopy) (Variables|/Game/FPS_Assault_Pack/Blueprints/RU74/BP_RU74_Character.BP_RU74_Character_C|GetWeaponInv _returnvalue) (Variables|/Game/FPS_Assault_Pack/Blueprints/RU74/BP_RU74_Character.BP_RU74_Character_C|GetWeaponNumber _returnvalue))) (Variables|Default|GetMaxReserveAmmo)))
      (if (Variables|Default|GetOverlap)
        (Development|PrintString "Hello")
        (if (>= (Variables|/Game/FPS_Assault_Pack/Blueprints/RU74/BP_RU74_Character.BP_RU74_Character_C|GetPoints _returnvalue) _requiredpoints)
          ;[1 1 1] Set spare ammo and remove points
          (Utilities|Struct|SetmembersinWeaponsInfo (Utilities|Array|Get(acopy) (Variables|/Game/FPS_Assault_Pack/Blueprints/RU74/BP_RU74_Character.BP_RU74_Character_C|GetWeaponInv _returnvalue) (Variables|/Game/FPS_Assault_Pack/Blueprints/RU74/BP_RU74_Character.BP_RU74_Character_C|GetWeaponNumber _returnvalue)) (+ (Utilities|Struct|BreakWeaponsInfo (Utilities|Array|Get(acopy) (Variables|/Game/FPS_Assault_Pack/Blueprints/RU74/BP_RU74_Character.BP_RU74_Character_C|GetWeaponInv _returnvalue) (Variables|/Game/FPS_Assault_Pack/Blueprints/RU74/BP_RU74_Character.BP_RU74_Character_C|GetWeaponNumber _returnvalue))) (Variables|Default|GetAddAmmo)))
          (Variables|/Game/FPS_Assault_Pack/Blueprints/RU74/BP_RU74_Character.BP_RU74_Character_C|SetPoints _returnvalue (- (Variables|/Game/FPS_Assault_Pack/Blueprints/RU74/BP_RU74_Character.BP_RU74_Character_C|GetPoints _returnvalue) _requiredpoints)))))))

(fn ConstructionScript)