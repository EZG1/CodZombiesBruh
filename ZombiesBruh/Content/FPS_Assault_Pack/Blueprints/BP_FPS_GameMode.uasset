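; FPS game mode that runs round-based zombie spawning across the map's SpawnPoint actors.
; On BeginPlay it caches all spawn points and starts a looping one-second timer.
; Each tick below the on-map zombie cap spawns an enemy at a random point, unless the round's kill target is met.
; Meeting that target pauses spawning for a 20-second delay, then resets kills and increments the round.
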(event Custom|ActivateSpawner
  (bind _spawnerlist (Variables|Default|GetSpawnerList))
  ;[1 1 1] Creating a list of all spawnpoints
  ;[1 1 1] Checking if too many zombies are on the map
  (if (not (== (Variables|Default|GetZombies%20on%20map) (Variables|Default|GetMaxZombieCount)))
    ;[1 1 1] Checking killed zombies for next round
    (if (>= (Variables|Default|GetZombiesKilledThisRound) (Variables|Default|GetZombiesNeededForNextRound))
      ;[1 1 1] Wait 20 seconds, move round count forward
      (Utilities|FlowControl|Delay 2e+01)
      (Variables|Default|SetZombiesKilledThisRound 0)
      (Variables|Default|SetRoundCount (+ (Variables|Default|GetRoundCount) 1))
      (else
        ;[1 1 1] Spawn zombie, +1 to zombie count on map
        (Default|SpawnEnemy (Utilities|Array|Get(acopy) _spawnerlist (Math|Random|RandomIntegerinRange 0 (- (Utilities|Array|Length _spawnerlist) 1))))
        (Variables|Default|SetZombies%20on%20map (+ (Variables|Default|GetZombies%20on%20map) 1))))))

(event EventBeginPlay
  ;[1 1 1] Creating a list of all spawnpoints
  (bind _outactors (Actor|GetAllActorsOfClass "/Game/AI/SpawnPoint.SpawnPoint_C"))
  (Variables|Default|SetSpawnerList _outactors)
  (Utilities|Time|SetTimerbyEvent (delegate Custom|ActivateSpawner) 1.0 true))

(fn ConstructionScript)